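; BP_ClickMovePlayerController is a player controller that moves the controlled pawn toward the mouse cursor while the left mouse button is held.
; The LeftClick input sets a held flag, and Tick traces under the cursor on the Visibility channel each frame while it is set.
; The hit location goes to SimpleMoveToLocation, but only when it lies beyond a short minimum distance from the pawn.
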(event `self.ReceiveTick`
  (params (DeltaSeconds :type "Float (single-precision)"))
  (if (`self.bClickLeftMouse`)
    (`self.MoveToMouseCursor`)))

(event `InputAction|LeftClick`
  (params (Key :type "Key Structure"))
  (:`Pressed`
    (`self.InputLeftMouseButtonPressed`))
  (:`Released`
    (`self.InputLeftMouseButtonReleased`)))

(fn `InputLeftMouseButtonPressed`
  (set `self.bClickLeftMouse` true))

(fn `InputLeftMouseButtonReleased`
  (set `self.bClickLeftMouse` false))

(fn `MoveToMouseCursor`
  (bind (_hitresult _returnvalue) (`self.GetHitResultUnderCursorByChannel` self "TraceTypeQuery1" true))
  (if _returnvalue
    (`self.SetNewDestination` (`.Location` (`GameplayStatics.BreakHitResult` _hitresult)))))

(fn `SetNewDestination`
  (params (NewDestination :type "Vector Structure"))
  (if (> (`KismetMathLibrary.Vector_Distance` NewDestination (`self.K2_GetActorLocation` (`self.K2_GetPawn`))) 120.0)
    (`AIBlueprintHelperLibrary.SimpleMoveToLocation` self NewDestination)))

(fn `UserConstructionScript`)