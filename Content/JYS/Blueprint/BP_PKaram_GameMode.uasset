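; Game mode that sets up the goal-point HUD and handles player respawning.
; On BeginPlay it adds the WBP_GoalPoint widget to the viewport, shows the mouse cursor and copies PlayerPoint into PlayerHasPoint.
; Its PlayerRespawn event finds the BP_location actor, waits briefly, then spawns a BP_player at that transform and has the first player controller possess it.
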(event `self.ReceiveBeginPlay`
  (bind _returnvalue (`|CreateWidget` "/Game/Main/UI/WBP_GoalPoint.WBP_GoalPoint_C"))
  (`UserWidget.AddToViewport` _returnvalue 0)
  (set `PlayerController.bShowMouseCursor` true (`GameplayStatics.GetPlayerController` 0))
  (set `self.PlayerHasPoint` (`self.PlayerPoint`)))

(event `self.ReceiveTick`
  (params (DeltaSeconds :type "Float (single-precision)")))

(event `PlayerRespawn`
  (bind _returnvalue (`GameplayStatics.GetActorOfClass` "/Game/JYS/Blueprint/BP_location.BP_location_C"))
  (`KismetSystemLibrary.Delay` 2.0)
  (bind _returnvalue_2 (`|SpawnActorFromClass` "/Game/JYS/Blueprint/BP_player.BP_player_C" (`self.GetTransform` _returnvalue) "Undefined" "MultiplyWithRoot" null null))
  (`Controller.Possess` (`GameplayStatics.GetPlayerController` 0) _returnvalue_2))

(fn `UserConstructionScript`)