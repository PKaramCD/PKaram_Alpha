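; Player Blueprint for a ball-collecting game with combat, health and respawn.
; CheckTargetColl overlaps store the target and tag flags: Space collects balls, key 1 in a Zone subtracts Itemcount from the GameMode's PlayerHasPoint and decrements it.
; The attack input damages the first actor of the target's class if it is a BP_EnemyBase.
; AnyDamage lowers Hp; destruction triggers GameMode respawn and drops a BP_ball.
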(event `InputAction|attack`
  (params (Key :type "Key Structure"))
  ;[1 1 1] Q누르면 공격 Enemy랑 NEnemy 공격
)

(event `self.ReceiveActorBeginOverlap`
  (params (OtherActor :type "Actor Object Reference")))

(event `self.ReceiveBeginPlay`
  ;[1 1 1] 플레이어가 태어날 때 HP에 MaxHP 값을 Set하고싶다.
  (set `self.Hp` (`self.MaxHP`))
  (bind _returnvalue (`|CreateWidget` "/Game/JYS/UI/WBP_Counter.WBP_Counter_C"))
  (`UserWidget.AddToViewport` _returnvalue 0)
  (set `self.HasWidget` false))

(event `InputAction|attack`
  (params (Key :type "Key Structure"))
  ;[1 1 1] Q누르면 공격
  (:`Pressed`
    (bind _returnvalue (`GameplayStatics.GetActorOfClass` (`GameplayStatics.GetObjectClass` (`self.Target`))))
    (bind _asbp_enemy_base (cast `/Game/KMS/Blueprints/BP_EnemyBase` _returnvalue))
    (`GameplayStatics.ApplyDamage` _asbp_enemy_base (`self.Damage`))))

(event `self.ReceiveTick`
  (params (DeltaSeconds :type "Float (single-precision)")))

(event `Key|One`
  (params (Key :type "Key Structure"))
  ;[1 1 1] Zone에서 볼 카운트 --
  (:`Pressed`
    (if (and (> (`self.Itemcount`) 0) (`self.Zone`))
      (bind _asbp_pkaram_game_mode (cast `/Game/JYS/Blueprint/BP_PKaram_GameMode` (`GameplayStatics.GetGameMode`)))
      (set `/Game/JYS/Blueprint/BP_PKaram_GameMode.PlayerHasPoint` (- (`/Game/JYS/Blueprint/BP_PKaram_GameMode.PlayerHasPoint` _asbp_pkaram_game_mode) (`self.Itemcount`)) _asbp_pkaram_game_mode)
      (bind _result (`/Engine/EditorBlueprintResources/StandardMacros.DecrementInt` (`self.Itemcount`))
        (:`  `
          (set `self.Itemcount` _result))))))

(event `self.CheckTargetColl.OnComponentBeginOverlap`
  (params (OverlappedComponent :type "PrimitiveComponent Object Reference") (OtherActor :type "Actor Object Reference") (OtherComp :type "PrimitiveComponent Object Reference") (OtherBodyIndex :type Integer) (bFromSweep :type Boolean) (SweepResult :type "HitResult Structure (by ref)"))
  (`|ExecutionSequence`
    (:`then_0`
      (set `self.Zone` (`self.ActorHasTag` OtherActor "Zone"))
      (bind _output_get (set `self.Target` OtherActor))
      (`KismetSystemLibrary.PrintString` (`KismetSystemLibrary.GetDisplayName` _output_get)))
    (:`then_1`
      (set `self.isBall` (`self.ActorHasTag` OtherActor "Ball")))
    (:`then_2`
      (set `self.IsEnemy` (`self.ActorHasTag` OtherActor "Enemy")))
    (:`then_3`
      ;[1 1 1] HP가 0일때 죽고 부활
      (if (== (`self.Hp`) 0.0)
        (`self.K2_DestroyActor`)))
    (:`then_4`
      (set `self.IsNEnemy` (`self.ActorHasTag` OtherActor "NEnemy")))))

(event `self.ReceiveActorEndOverlap`
  (params (OtherActor :type "Actor Object Reference"))
  (`|ExecutionSequence`
    (:`then_0`
      (set `self.isBall` false))
    (:`then_1`
      (set `self.Zone` false))))

(event `self.ReceiveDestroyed`
  ;[1 1 1] HP가 0일때 죽고 부활
  (bind _asbp_pkaram_game_mode (cast `/Game/JYS/Blueprint/BP_PKaram_GameMode` (`GameplayStatics.GetGameMode`)))
  (`/Game/JYS/Blueprint/BP_PKaram_GameMode.PlayerRespawn` _asbp_pkaram_game_mode)
  (`|SpawnActorFromClass` "/Game/JYS/Blueprint/BP_ball.BP_ball_C" (`SceneComponent.K2_GetComponentToWorld` (`self.P_DropItemPos`)) "Undefined" "MultiplyWithRoot" null null))

(event `Key|SpaceBar`
  (params (Key :type "Key Structure"))
  ;[1 1 1] spacebar를 눌렀을 때 balls 카운트 +1
  (:`Pressed`
    (if (`self.isBall`)
      (`self.K2_DestroyActor` (`self.Target`))
      (`/Engine/EditorBlueprintResources/StandardMacros.IncrementInt` (`self.Itemcount`)))))

(event `Key|Five`
  (params (Key :type "Key Structure")))

(event `self.ReceiveAnyDamage`
  (params (Damage :type "Float (single-precision)") (DamageType :type "DamageType Object Reference") (InstigatedBy :type "Controller Object Reference") (DamageCauser :type "Actor Object Reference"))
  ;[1 1 1] Take Damage
  (if (> (`self.Hp`) 0.0)
    (set `self.Hp` (- (`self.Hp`) Damage))
    (`KismetSystemLibrary.PrintString` "Damaged!!!")
    (else
      (`self.K2_DestroyActor`))))

(fn `MyApplyDamage`
  (params (Damage :type Integer))
  (returns (`Result HP` :type "Float (double-precision)"))
  (set `self.Hp` (- (`self.Hp`) Damage))
  (return (`self.Hp`)))

(fn `UserConstructionScript`)