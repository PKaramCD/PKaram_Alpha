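; Base enemy that fights Player and NEnemy actors, tracks health and drops a BP_ball when destroyed.
; TargetCheckCollision_E overlaps set AI blackboard target flags, while capsule overlaps toggle delayed Tick damage.
; Targets resolve via GetActorOfClass on the overlapped class, so the first instance found is used.
; Damage taken at depleted health destroys it and clears BP_EnemySpawn's HasEnemy; PawnSensing and sphere-overlap attack logic are disconnected.
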(event `self.ReceiveBeginPlay`
  (set `self.EnemyHealth` (`self.MaxEnemyHealth`))
  (set `self.IsDead` false)
  (set `self.HasBallCount` 0))

(event `self.ReceiveActorBeginOverlap`
  (params (OtherActor :type "Actor Object Reference")))

(event `self.ReceiveTick`
  (params (DeltaSeconds :type "Float (single-precision)"))
  (if (`self.CanAttack`)
    (`KismetSystemLibrary.Delay` 1.0)
    (`GameplayStatics.ApplyDamage` (`self.Target_Characters`) 10.0)
    (`KismetSystemLibrary.Delay` 1.0)))

(event `self.CapsuleComponent.OnComponentBeginOverlap`
  (params (OverlappedComponent :type "PrimitiveComponent Object Reference") (OtherActor :type "Actor Object Reference") (OtherComp :type "PrimitiveComponent Object Reference") (OtherBodyIndex :type Integer) (bFromSweep :type Boolean) (SweepResult :type "HitResult Structure (by ref)"))
  ;[1 1 1] Attack
  (if (`self.ActorHasTag` OtherActor "Player")
    (bind _returnvalue (`GameplayStatics.GetActorOfClass` (`GameplayStatics.GetObjectClass` OtherActor)))
    (bind _output_get (set `self.Target_Characters` _returnvalue))
    (bind _ascharacter (cast `Character` _output_get))
    (bind _output_get_2 (set `self.CanAttack` true))
    (if _output_get_2
      (`BlackboardComponent.SetValueAsBool` (`AIBlueprintHelperLibrary.GetBlackboard` (`AIBlueprintHelperLibrary.GetAIController` self)) "CheckEnemyDeadState" true))
    (elif (`self.ActorHasTag` OtherActor "NEnemy")
      (bind _returnvalue_2 (`GameplayStatics.GetActorOfClass` (`GameplayStatics.GetObjectClass` OtherActor)))
      (bind _output_get_3 (set `self.Target_Characters` _returnvalue_2))
      (bind _ascharacter_2 (cast `Character` _output_get_3))
      (set `self.CanAttack` true))))

(event `self.PawnSensing.OnSeePawn`
  (params (Pawn :type "Pawn Object Reference"))
  ;[1 1 1] Comment
)

(event `self.CapsuleComponent.OnComponentEndOverlap`
  (params (OverlappedComponent :type "PrimitiveComponent Object Reference") (OtherActor :type "Actor Object Reference") (OtherComp :type "PrimitiveComponent Object Reference") (OtherBodyIndex :type Integer))
  ;[1 1 1] Comment
  (if (`self.ActorHasTag` OtherActor "Player")
    (bind _returnvalue (`GameplayStatics.GetActorOfClass` (`GameplayStatics.GetObjectClass` OtherActor)))
    (bind _output_get (set `self.Target_Characters` _returnvalue))
    (cast `Character` _output_get)
    (set `self.CanAttack` false)
    (set `self.Target_Characters` null)
    (elif (`self.ActorHasTag` OtherActor "NEnemy")
      (bind _returnvalue_2 (`GameplayStatics.GetActorOfClass` (`GameplayStatics.GetObjectClass` OtherActor)))
      (bind _output_get_2 (set `self.Target_Characters` _returnvalue_2))
      (cast `Character` _output_get_2)
      (set `self.CanAttack` false)
      (set `self.Target_Characters` null))))

(event `self.TargetCheckCollision_E.OnComponentBeginOverlap`
  (params (OverlappedComponent :type "PrimitiveComponent Object Reference") (OtherActor :type "Actor Object Reference") (OtherComp :type "PrimitiveComponent Object Reference") (OtherBodyIndex :type Integer) (bFromSweep :type Boolean) (SweepResult :type "HitResult Structure (by ref)"))
  ;[1 1 1] Comment
  (if (`self.ActorHasTag` OtherActor "Player")
    (bind _returnvalue (`GameplayStatics.GetActorOfClass` (`GameplayStatics.GetObjectClass` OtherActor)))
    (bind _output_get (set `self.CheckTarget` _returnvalue))
    (bind _ascharacter (cast `Character` _output_get))
    (`BlackboardComponent.SetValueAsBool` (`AIBlueprintHelperLibrary.GetBlackboard` (`AIBlueprintHelperLibrary.GetAIController` self)) "HasSeenTarget" true)
    (`BlackboardComponent.SetValueAsBool` (`AIBlueprintHelperLibrary.GetBlackboard` (`AIBlueprintHelperLibrary.GetAIController` self)) "HasSetTargetPlayer" true)
    (`BlackboardComponent.SetValueAsBool` (`AIBlueprintHelperLibrary.GetBlackboard` (`AIBlueprintHelperLibrary.GetAIController` self)) "HasSetTargetNEnemy" false)
    (elif (`self.ActorHasTag` OtherActor "NEnemy")
      (bind _returnvalue_2 (`GameplayStatics.GetActorOfClass` (`GameplayStatics.GetObjectClass` OtherActor)))
      (bind _output_get_2 (set `self.CheckTarget` _returnvalue_2))
      (bind _ascharacter_2 (cast `Character` _output_get_2))
      (`BlackboardComponent.SetValueAsBool` (`AIBlueprintHelperLibrary.GetBlackboard` (`AIBlueprintHelperLibrary.GetAIController` self)) "HasSeenTarget" true)
      (`BlackboardComponent.SetValueAsBool` (`AIBlueprintHelperLibrary.GetBlackboard` (`AIBlueprintHelperLibrary.GetAIController` self)) "HasSetTargetNEnemy" true)
      (`BlackboardComponent.SetValueAsBool` (`AIBlueprintHelperLibrary.GetBlackboard` (`AIBlueprintHelperLibrary.GetAIController` self)) "HasSetTargePlayer" false)
      (elif (`self.ActorHasTag` "Ball")
        _))))

(event `self.TargetCheckCollision_E.OnComponentEndOverlap`
  (params (OverlappedComponent :type "PrimitiveComponent Object Reference") (OtherActor :type "Actor Object Reference") (OtherComp :type "PrimitiveComponent Object Reference") (OtherBodyIndex :type Integer))
  ;[1 1 1] Comment
  (if (`self.ActorHasTag` OtherActor "Player")
    (bind _returnvalue (`GameplayStatics.GetActorOfClass` (`GameplayStatics.GetObjectClass` OtherActor)))
    (bind _output_get (set `self.CheckTarget` _returnvalue))
    (cast `Character` _output_get)
    (`BlackboardComponent.SetValueAsBool` (`AIBlueprintHelperLibrary.GetBlackboard` (`AIBlueprintHelperLibrary.GetAIController` self)) "HasSeenTarget" false)
    (`BlackboardComponent.SetValueAsBool` (`AIBlueprintHelperLibrary.GetBlackboard` (`AIBlueprintHelperLibrary.GetAIController` self)) "HasSetTargetPlayer" false)
    (`BlackboardComponent.SetValueAsBool` (`AIBlueprintHelperLibrary.GetBlackboard` (`AIBlueprintHelperLibrary.GetAIController` self)) "HasSetTargetNEnemy" false)
    (`BlackboardComponent.SetValueAsBool` (`AIBlueprintHelperLibrary.GetBlackboard` (`AIBlueprintHelperLibrary.GetAIController` self)) "CanAttackPlayer" false)
    (set `self.CheckTarget` null)
    (set `self.Target_Characters` null)
    (elif (`self.ActorHasTag` OtherActor "NEnemy")
      (bind _returnvalue_2 (`GameplayStatics.GetActorOfClass` (`GameplayStatics.GetObjectClass` OtherActor)))
      (bind _output_get_2 (set `self.CheckTarget` _returnvalue_2))
      (bind _ascharacter (cast `Character` _output_get_2))
      (`BlackboardComponent.SetValueAsBool` (`AIBlueprintHelperLibrary.GetBlackboard` (`AIBlueprintHelperLibrary.GetAIController` self)) "HasSeenTarget" false)
      (`BlackboardComponent.SetValueAsBool` (`AIBlueprintHelperLibrary.GetBlackboard` (`AIBlueprintHelperLibrary.GetAIController` self)) "HasSetTargetNEnemy" false)
      (`BlackboardComponent.SetValueAsBool` (`AIBlueprintHelperLibrary.GetBlackboard` (`AIBlueprintHelperLibrary.GetAIController` self)) "HasSetTargePlayer" false))))

(event `self.ReceiveAnyDamage`
  (params (Damage :type "Float (single-precision)") (DamageType :type "DamageType Object Reference") (InstigatedBy :type "Controller Object Reference") (DamageCauser :type "Actor Object Reference"))
  ;[1 1 1] Take Damage
  (if (> (`self.EnemyHealth`) 0.0)
    (set `self.EnemyHealth` (- (`self.EnemyHealth`) Damage))
    (`KismetSystemLibrary.PrintString` "Damaged!!!")
    (else
      (`self.K2_DestroyActor`)
      (set `self.IsDead` true)
      (bind _returnvalue (`GameplayStatics.GetActorOfClass` "/Game/KMS/Blueprints/BP_EnemySpawn.BP_EnemySpawn_C"))
      (set `/Game/KMS/Blueprints/BP_EnemySpawn.HasEnemy` false _returnvalue)
      (`BlackboardComponent.SetValueAsBool` (`AIBlueprintHelperLibrary.GetBlackboard` (`AIBlueprintHelperLibrary.GetAIController` self)) "CheckEnemyDeadState" true))))

(event `self.ReceiveDestroyed`
  ;[1 1 1] DropItem
  (`|SpawnActorFromClass` "/Game/JYS/Blueprint/BP_ball.BP_ball_C" (`SceneComponent.K2_GetComponentToWorld` (`self.DropItemPos`)) "Undefined" "MultiplyWithRoot" null null))

(fn `UserConstructionScript`)