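; BP_Nuetral is an AI pawn that wanders until it spots a pawn, then moves toward the player.
; On BeginPlay it sets health to max and loops AI MoveTo calls to random reachable nearby points.
; PawnSensing triggers the chase, whose arrival only toggles a CanAttack flag, with no attack performed.
; Myapplydamage subtracts damage and returns the remaining health, with no death handling.
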(event `self.ReceiveBeginPlay`
  (`self.Roam Around`)
  (set `self.health` (`self.Maxhealth`)))

(event `self.PawnSensing.OnSeePawn`
  (params (Pawn :type "Pawn Object Reference"))
  (set `self.isSeeingPlayer?` true)
  (`self.FollowPlayer`))

(event `FollowPlayer`
  (set `self.canAttack?` true)
  (if (`self.isSeeingPlayer?`)
    (`|AIMoveTo` self (0.0 0.0 0.0) (`GameplayStatics.GetPlayerCharacter` 0) 70.0
      (:`OnSuccess`
        (if (`self.canAttack?`)
          (set `self.canAttack?` false)
          (`KismetSystemLibrary.Delay` 0.2)
          (set `self.canAttack?` false))))
    (else
      (set `self.isSeeingPlayer?` false))))

(event `Roam Around`
  ;[1 1 1] Roam Around
  (`|AIMoveTo` self (`NavigationSystemV1.K2_GetRandomReachablePointInRadius` (`self.K2_GetActorLocation`) 500.0 null null) null 120.0
    (:`OnSuccess`
      (`KismetSystemLibrary.Delay` 1.2)
      (`self.Roam Around`))))

(fn `Myapplydamage`
  (params (Damage :type "Float (double-precision)"))
  (returns (NewParam :type "Float (double-precision)"))
  (set `self.health` (- (`self.health`) Damage))
  (return (`self.health`)))

(fn `UserConstructionScript`)